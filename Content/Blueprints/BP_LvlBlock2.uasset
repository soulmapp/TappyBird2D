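; Level actor for a Flappy Bird-style Tappy Chicken minigame, owning the side-view camera, bird, scrolling scenery and obstacles.
; Click or touch starts obstacle panning and replays a flap timeline, whose curves drive the bird's height and pitch on Tick.
; Background sprites and obstacles scroll left and wrap for endless motion, with obstacle heights randomized.
; Flash halts the bird, input and obstacles, and animates a screen flash through a Material Parameter Collection.
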(event Custom|EventStartGame
  ;[1 1 1] STart Game
  (if (Variables|Default|GetCanInput)
    (Variables|Default|SetCanInput true)
    (Development|PrintString "can score")
    (Variables|Default|SetCanScore true)))

(event Custom|Flash
  ;[1 1 1] Flash - Flashes the screen and stops all panning on the materials, and obstacles
  (Variables|Default|SetCanPanObstacles false)
  (Variables|Default|SetCanInput false)
  (Variables|Default|SetCanScore false)
  (Audio|Components|Audio|Stop (Variables|Default|GetTappyBIrd2d))
  (Utilities|FlowControl|Sequence
    (:then_0
      (bind _flash (Timeline|Timeline_Flash PlayFromStart)
        (:Update
          (Rendering|Material|SetScalarParameterValue "/Game/Materials/MPC_TappyChicken_01.MPC_TappyChicken_01" "ScreenFlashAmmount" _flash :!class /Script/Engine.KismetMaterialLibrary))))
    (:then_1
      (for _array_element (Variables|Default|GetActiveObstacles)
        (bind _asbp_obstacle_post_c (Utilities|Casting|CastToBP_Obstacle_Post _array_element))
        (Variables|/Game/Blueprints/BP_Obstacle_Post.BP_Obstacle_Post_C|SetCanMove _asbp_obstacle_post_c false)))))

(event Custom|FlapTappy
  ;[1 1 1] Flap - Animates the upward movement of the chicken when you tap.
  (Audio|PlaySoundatLocation "/Game/Audio/SFX_FlapWing_Cue.SFX_FlapWing_Cue" "0, 0, 0")
  (bind (_direction _vertmovement _rotation) (Timeline|Timeline_0 PlayFromStart)))

(event EventBeginPlay
  (bind _returnvalue (Game|GetPlayerController 0))
  (bind (_sizex _sizey) (HUD|GetViewportSize _returnvalue))
  ;[1 1 1] Setup Camera and Initial Setup
  (Variables|/Script/Engine.CameraComponent|SetOrthoWidth (Variables|Default|GetCamera1) (Math|Float|Clamp(Float) (/ (* _sizex 4e+03) (* _sizey 0.75)) 1.28e+03 8e+03))
  (Game|Player|SetViewTargetwithBlend _returnvalue self 0.0 "VTBlend_Linear" 0.0 false)
  (Variables|Default|SetGameMode "NewEnumerator0")
  (Utilities|FlowControl|Sequence
    (:then_0
      (Utilities|Array|Clear (Variables|Default|GetActiveObstacles))
      (Variables|Default|SetIsRetry false)
      (CallFunction|ResetObstacles))))

(event EventTick
  (params (DeltaSeconds :type Float%20%28single-precision%29))
  (bind _tappybird2d (Variables|Default|GetTappyBIrd2d))
  ;[1 1 1] Flap - Animates the upward movement of the chicken when you tap.
  (Variables|Default|SetDeltaTime DeltaSeconds)
  (Utilities|FlowControl|Sequence
    (:then_0
      (if (Audio|Components|Audio|IsPlaying (Variables|Default|GetTappyBIrd2d))
        (CallFunction|PanLayers))
      (if (Variables|Default|GetCanPanObstacles)
        (CallFunction|PanObstacles))
      (Transformation|SetRelativeLocation _tappybird2d (Math|Vector|MakeVector 0.0 2.9e+02 (+ (.Z (Math|Vector|BreakVector (Transformation|GetWorldLocation _tappybird2d))) (* (* (stale Custom|FlapTappy _vertmovement) 5e+02) (Variables|Default|GetDeltaTime)))) false)
      (Transformation|SetWorldRotation _tappybird2d (Math|Interpolation|RInterpTo (Transformation|GetWorldRotation _tappybird2d) (Class|KismetMathLibrary|MakeRot (stale Custom|FlapTappy _rotation) 0.0 0.0) (Variables|Default|GetDeltaTime) 1.0) false))
    (:then_1
      ;[1 1 1] STart Game
      (if (Variables|Default|GetCanInput)
        (Variables|Default|SetCanInput true)
        (Development|PrintString "can score")
        (Variables|Default|SetCanScore true)))))

(event EventToggleStartGame
  (params (CanInput :type Boolean))
  ;[1 1 1] Also tried
  (Variables|Default|SetCanInput CanInput))

(event Input|MouseEvents|LeftMouseButton
  ;[1 1 1] Tap Tappy Bird
  (:Pressed
    (if (Variables|Default|GetCanInput)
      (Variables|Default|SetGameMode "NewEnumerator1")
      (switch Utilities|FlowControl|Switch|SwitchonGameMode_Enum (Variables|Default|GetGameMode)
        (:NewEnumerator1
          (Variables|Default|SetGameMode "NewEnumerator2")
          (Variables|Default|SetCanPanObstacles true)
          (CallFunction|FlapTappy))
        (:NewEnumerator2
          (CallFunction|FlapTappy))))))

(event Input|TouchEvents|InputTouch
  (params (Location :type Vector) (FingerIndex :type ETouchIndex%20Enum))
  ;[1 1 1] Tap Tappy Bird
  (:Pressed
    (if (Variables|Default|GetCanInput)
      (Variables|Default|SetGameMode "NewEnumerator1")
      (switch Utilities|FlowControl|Switch|SwitchonGameMode_Enum (Variables|Default|GetGameMode)
        (:NewEnumerator1
          (Variables|Default|SetGameMode "NewEnumerator2")
          (Variables|Default|SetCanPanObstacles true)
          (CallFunction|FlapTappy))
        (:NewEnumerator2
          (CallFunction|FlapTappy))))))

(fn ConstructionScript
  (bind _panninglayersprites (Variables|Default|GetPanningLayerSprites))
  (Utilities|Array|Clear (Variables|Default|GetPanningLayerSprites))
  (Utilities|Array|Add _panninglayersprites (Variables|Default|GetCllouds))
  (Utilities|Array|Add _panninglayersprites (Variables|Default|GetBushes))
  (Utilities|Array|Add _panninglayersprites (Variables|Default|GetGround)))

(fn PanObstacles
  (bind _canobstaclescore (Variables|Default|GetCanObstacleScore))
  (for (_array_element _array_index) (Variables|Default|GetPanningObstacles)
    (if (< (.X (Math|Vector|BreakVector (Variables|/Script/Engine.SceneComponent|GetRelativeLocation _array_element))) 0.0)
      (if (Utilities|Array|Get(acopy) _canobstaclescore _array_index)
        (Utilities|Array|SetArrayElem _canobstaclescore _array_index false)))
    (if (< (.X (Math|Vector|BreakVector (Variables|/Script/Engine.SceneComponent|GetRelativeLocation _array_element))) 0.0)
      (Utilities|Array|SetArrayElem (Variables|Default|GetCanObstacleScore) _array_index true)
      (Transformation|AddRelativeLocation _array_element "1500.000000,170.000000, 0" false)
      (Transformation|SetRelativeLocation _array_element (Math|Vector|MakeVector (.X (Math|Vector|BreakVector (Variables|/Script/Engine.SceneComponent|GetRelativeLocation _array_element))) 1.7e+02 (+ 3.1e+02 (Math|Random|RandomFloatinRange -256.0 256.0))) false))
    (Transformation|AddRelativeLocation _array_element (Math|Vector|MakeVector (* (* (* 0.08 (Variables|Default|GetDeltaTime)) 4e+03) -1.0) 0.0 0.0) false)))

(fn PanLayers
  (for (_array_element _array_index) (Variables|Default|GetPanningLayerSprites)
    (if (< (.X (Math|Vector|BreakVector (Variables|/Script/Engine.SceneComponent|GetRelativeLocation _array_element))) -4096.0)
      (Transformation|AddRelativeLocation _array_element "4096.000000, 0, 0" false))
    (Transformation|AddRelativeLocation _array_element (Math|Vector|MakeVector (* (* (* (Utilities|Array|Get(acopy) (Variables|Default|GetPanningLayerTimes) _array_index) (Variables|Default|GetDeltaTime)) 4e+03) -1.0) 0.0 0.0) false)))

(fn ResetObstacles
  (bind _canobstaclescore (Variables|Default|GetCanObstacleScore))
  (for (_array_element _array_index) (Variables|Default|GetPanningObstacles)
    (Transformation|SetRelativeLocation _array_element (Math|Vector|MakeVector (Math|Conversions|ToFloat(Integer) (+ 3072 (* _array_index 800))) 1.7e+02 (+ 3.1e+02 (Math|Random|RandomFloatinRange -256.0 256.0))) false))
  (for (_ _array_index_2) _canobstaclescore
    (Utilities|Array|SetArrayElem _canobstaclescore _array_index_2 true)))