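; BP_Obstacle_Post is a moving obstacle that awards a point once it passes a fixed world X threshold.
; While CanMove is true, Tick sweeps it along its local Y axis at MovementAmount per second.
; On first crossing the threshold, a DoOnce casts GameManager to BP_LvlBlock and calls Score.
; The construction script gives the ArrowOffset component a random vertical position at a fixed local Y offset.
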(event EventTick
  (params (DeltaSeconds :type Float%20%28single-precision%29))
  (Variables|Default|SetDeltaTime DeltaSeconds)
  (if (Variables|Default|GetCanMove)
    (Transformation|AddActorLocalOffset (Math|Vector|MakeVector 0.0 (* (Variables|Default|GetMovementAmount) (Variables|Default|GetDeltaTime)) 0.0) true)
    (if (< (.X (Math|Vector|BreakVector (Transformation|GetActorLocation))) -195.0)
      (Utilities|FlowControl|DoOnce false
        (:Completed
          (bind _asbp_lvlblock_c (Utilities|Casting|CastToBP_LvlBlock (Variables|Default|GetGameManager)))
          (Default|Score _asbp_lvlblock_c))))))

(fn ConstructionScript
  (Transformation|SetRelativeLocation (Variables|Default|GetArrowOffset) (Math|Vector|MakeVector 0.0 1.7e+02 (Math|Random|RandomFloatinRange -256.0 256.0)) false))