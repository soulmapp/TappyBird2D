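; Hot air balloon sprite Blueprint, set up to move and scale the HotBallon component along a timeline.
; An unconnected movement timeline lerps from current world location toward EndPoint, but never runs as nothing triggers it.
; Its StartScale-to-EndScale lerp also feeds SetRelativeLocation, so it overwrites the position instead of scaling.
; The construction script rebuilds the three vectors from their own components, leaving them unchanged.
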(fn ConstructionScript
  (Variables|Default|SetEndPoint (Math|Vector|MakeVector (.X (Math|Vector|BreakVector (Variables|Default|GetEndPoint))) (.Y (Math|Vector|BreakVector (Variables|Default|GetEndPoint))) (.Z (Math|Vector|BreakVector (Variables|Default|GetEndPoint)))))
  (Variables|Default|SetStartScale (Math|Vector|MakeVector (.X (Math|Vector|BreakVector (Variables|Default|GetStartScale))) (.Y (Math|Vector|BreakVector (Variables|Default|GetStartScale))) (.Z (Math|Vector|BreakVector (Variables|Default|GetStartScale)))))
  (Variables|Default|SetEndScale (Math|Vector|MakeVector (.X (Math|Vector|BreakVector (Variables|Default|GetEndScale))) (.Y (Math|Vector|BreakVector (Variables|Default|GetEndScale))) (.Z (Math|Vector|BreakVector (Variables|Default|GetEndScale))))))