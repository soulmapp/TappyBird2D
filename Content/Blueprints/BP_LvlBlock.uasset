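; Main game actor for Tappy Chicken, a 2D Flappy Bird-style game, owning camera, bird, scenery, menus, score and saves.
; Tick scrolls and recycles background sprites and randomized obstacles, scoring as obstacles pass the bird.
; Taps restart a timeline driving flap height and pitch; overlaps trigger a screen flash, crash and score-indexed egg award.
; High score and found eggs persist to a save slot, with high score also using leaderboards.
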(event OnComponentBeginOverlap(PowerUpTrigger)
  (params (OtherActor :type Actor%20Object%20Reference) (OtherComp :type Primitive%20Component%20Object%20Reference) (OtherBodyIndex :type Integer) (bFromSweep :type Boolean) (SweepResult :type Hit%20Result%20Structure%20%28by%20ref%29))
  ;[1 1 1] Power Up Collision Pickup
  (if (> (Variables|scoreboard|GetCurrentScore) 1)
    (Utilities|FlowControl|DoOnce false
      (:Completed
        (Development|PrintString "You Hvae picked up a pickup")
        (Audio|PlaySoundatLocation "/Game/Audio/popdissappear_Cue.popdissappear_Cue" "0, 0, 0")))))

(event OnComponentBeginOverlap(Sphere1)
  (params (OtherActor :type Actor%20Object%20Reference) (OtherComp :type Primitive%20Component%20Object%20Reference) (OtherBodyIndex :type Integer) (bFromSweep :type Boolean) (SweepResult :type Hit%20Result%20Structure%20%28by%20ref%29))
  ;[1 1 1] When the Chicken hits an Obstacle and to agnore power up collision box
  (if (not (Components|ComponentHasTag OtherComp (Utilities|Array|Get(acopy) (Variables|/Script/Engine.ActorComponent|GetComponentTags (Variables|Default|GetPowerUpTrigger)))))
    (if (< (.Z (Math|Vector|BreakVector (Transformation|GetWorldLocation (Variables|Character|GetTappyBIrd2d)))) -7e+02)
      (Utilities|FlowControl|DoOnce false
        (:Completed
          (CallFunction|Flash)
          (CallFunction|HitGorund)))
      (else
        (Utilities|FlowControl|DoOnce false
          (:Completed
            (CallFunction|Flash)
            (CallFunction|Crash)))))))

(event Custom|ResetGame
  (bind _tappybird2d (Variables|Character|GetTappyBIrd2d))
  ;[1 1 1] Reset Game.. Retry
  (for _array_element (Variables|Arrays|GetPanningLayerSprites)
    (Transformation|SetRelativeLocation _array_element (Math|Vector|MakeVector (.X (Math|Vector|BreakVector (Variables|/Script/Engine.SceneComponent|GetRelativeLocation _array_element))) (.Y (Math|Vector|BreakVector (Variables|/Script/Engine.SceneComponent|GetRelativeLocation _array_element))) (.Z (Math|Vector|BreakVector (Variables|/Script/Engine.SceneComponent|GetRelativeLocation _array_element)))) false)
    (Transformation|SetRelativeLocation _tappybird2d "-1575.000000,290.000000, 0" false)
    (Transformation|SetRelativeRotation _tappybird2d "0, 0, 0" false)
    (Audio|Components|Audio|Play _tappybird2d)
    (Rendering|SetVisibility _tappybird2d true false)
    (Variables|scoreboard|SetCurrentScore 0)
    (Rendering|Components|TextRender|SetText (Variables|TextRender|GetText_ScoreTxt) (Utilities|String|ToString(Integer) (Variables|scoreboard|GetCurrentScore)))
    (CallFunction|ResetObstacles)
    (CallFunction|RestartHitCollisons)
    (CallFunction|BirdFlyinEvent)
    ;;[0.1311 1 0.09645] Changing BG Color
    (CallFunction|ChooseSkyColor)
    (Variables|scoreboard|SetNewHighScore false)
    (Rendering|SetVisibility (Variables|Sprites|Getegg) false false)))

(event Custom|EventStartGame
  ;[1 1 1] STart Game
  (Variables|Bool|SetCanInput true)
  (Variables|Bool|SetCanScore true)
  (Variables|Bool|SetREadyToPlay true)
  (Variables|Bool|SetCanPanObstacles true)
  ;[1 1 1] Score HUD ENabled
  (bind _returnvalue (Class|WidgetBlueprintLibrary|Create "/Game/Hud/ScoreHUD.ScoreHUD_C"))
  (Variables|umg_menu|SetScoreHUD _returnvalue)
  (UserInterface|Viewport|AddtoViewport (Variables|umg_menu|GetScoreHUD) false))

(event Custom|ClearSavedGameData
  (bind _tappy2dsavegameobject (Variables|SaveGame|GetTappy2dSaveGameObject))
  ;[1 1 1] SaveGame
  (bind _asbp_tappybird2dsavegame_c (Utilities|Casting|CastToBP_TappyBIrd2dSaveGame _tappy2dsavegameobject))
  (Variables|/Game/Blueprints/BP_TappyBIrd2dSaveGame.BP_TappyBIrd2dSaveGame_C|SetHighScore _asbp_tappybird2dsavegame_c 0)
  (Variables|scoreboard|SetHighScore 0)
  (for _index (range 0 63)
    (Utilities|Array|SetArrayElem (Variables|Arrays|GetFoundEggs) _index false))
  (Variables|/Game/Blueprints/BP_TappyBIrd2dSaveGame.BP_TappyBIrd2dSaveGame_C|SetFoundEggs _asbp_tappybird2dsavegame_c (Variables|Arrays|GetFoundEggs))
  (SaveGame|SaveGametoSlot _tappy2dsavegameobject "Tappy2DSlot")
  (Development|PrintString "Saved File Has Been Cleared"))

(event Custom|SetTappyStartPostion
  ;[1 1 1] Set Tappy into Starting Location
  (bind _tappybirdxlocation (Timeline|TappyStartPostion_Timeline PlayFromStart)
    (:Update
      (Transformation|SetRelativeLocation (Variables|Character|GetTappyBIrd2d) (Math|Vector|MakeVector _tappybirdxlocation 2.9e+02 0.0) false))))

(event Custom|Score
  ;[1 1 1] Score
  (if (Variables|Bool|GetCanScore)
    (Variables|scoreboard|SetCurrentScore (+ (Variables|scoreboard|GetCurrentScore) 1))
    (Rendering|Components|TextRender|SetText (Variables|TextRender|GetText_ScoreTxt) (Utilities|String|ToString(Integer) (Variables|scoreboard|GetCurrentScore)))
    (Audio|PlaySoundatLocation "/Game/Audio/SFX_Score_01_Cue.SFX_Score_01_Cue" "0, 0, 0" 0.3)))

(event Custom|HitGorund
  (bind _tappybird2d (Variables|Character|GetTappyBIrd2d))
  (bind _tappy2dsavegameobject (Variables|SaveGame|GetTappy2dSaveGameObject))
  (bind _tappy2dsavegameobject_2 (Variables|SaveGame|GetTappy2dSaveGameObject))
  ;[1 1 1] Hit Ground - Opens the Scoreboard, Unhides the Play, Leaderboards, and Rate buttons, checks score to see it if beat your high score etc.
  (Utilities|FlowControl|DoOnce false
    (:Completed
      (Audio|PlaySoundatLocation "/Game/Audio/SFX_HitGround_01_Cue.SFX_HitGround_01_Cue" "0, 0, 0")
      (Audio|Components|Audio|Stop _tappybird2d)
      (CallFunction|SpawnAward)
      (Effects|SpawnEmitteratLocation "/Game/Effects/FX_FeathersHit_01.FX_FeathersHit_01" "-195.000000,290.000000,-700.000000")
      (Rendering|SetVisibility _tappybird2d false false)
      (Variables|Enum|SetGameMode "NewEnumerator3")
      (Variables|Bool|SetREadyToPlay false)
      (Class|LeaderboardBlueprintLibrary|WriteLeaderboardInteger (Game|GetPlayerController 0) "HighScore" (Variables|scoreboard|GetCurrentScore))
      (Utilities|Array|SetArrayElem (Variables|Arrays|GetFoundEggs) (Variables|scoreboard|GetCurrentScore) true)
      (bind _asbp_tappybird2dsavegame_c (Utilities|Casting|CastToBP_TappyBIrd2dSaveGame _tappy2dsavegameobject_2))
      (Variables|/Game/Blueprints/BP_TappyBIrd2dSaveGame.BP_TappyBIrd2dSaveGame_C|SetFoundEggs _asbp_tappybird2dsavegame_c (Variables|Arrays|GetFoundEggs))
      (SaveGame|SaveGametoSlot _tappy2dsavegameobject_2 "Tappy2DSlot")
      (if (> (Variables|scoreboard|GetCurrentScore) (Variables|scoreboard|GetHighScore))
        (Variables|scoreboard|SetHighScore (Variables|scoreboard|GetCurrentScore))
        (Utilities|FlowControl|Sequence
          (:then_0
            (Variables|scoreboard|SetNewHighScore true))
          (:then_1
            (bind _asbp_tappybird2dsavegame_c_2 (Utilities|Casting|CastToBP_TappyBIrd2dSaveGame _tappy2dsavegameobject))
            (Variables|/Game/Blueprints/BP_TappyBIrd2dSaveGame.BP_TappyBIrd2dSaveGame_C|SetHighScore _asbp_tappybird2dsavegame_c_2 (Variables|scoreboard|GetHighScore))
            (SaveGame|SaveGametoSlot _tappy2dsavegameobject "Tappy2DSlot")))))))

(event Custom|SpawnAward
  (bind _egg (Variables|Sprites|Getegg))
  ;[1 1 1] Hit Ground - Opens the Scoreboard, Unhides the Play, Leaderboards, and Rate buttons, checks score to see it if beat your high score etc.
  (Rendering|Material|SetScalarParameterValue (Variables|DMI|GetMID_Egg) "FrameNumber" (Math|Conversions|ToFloat(Integer) (Math|Integer|Clamp(Integer) (Variables|scoreboard|GetCurrentScore) 0 63)) :!class /Script/Engine.MaterialInstanceDynamic)
  (Audio|PlaySoundatLocation "/Game/Audio/SFX_LastCluck_Cue.SFX_LastCluck_Cue" "0, 0, 0")
  (Utilities|FlowControl|Sequence
    (:then_0
      (Audio|PlaySoundatLocation "/Game/Audio/SFX_LayEgg_01_Cue.SFX_LayEgg_01_Cue" "0, 0,0.000000")
      (Rendering|SetVisibility _egg true false)
      (bind (_direction _eggz _eggx) (Timeline|Timeline_LayEgg PlayFromStart)
        (:Update
          (Transformation|SetRelativeLocation _egg (Math|Vector|MakeVector _eggx 2.9e+02 _eggz) false))))
    (:then_1
      (Utilities|FlowControl|Delay 2.0)
      (bind _returnvalue (Class|WidgetBlueprintLibrary|Create "/Game/Menus/GameOver.GameOver_C"))
      (UserInterface|Viewport|AddtoViewport _returnvalue false true true))
    (:then_2
      (Utilities|FlowControl|Delay 1.5)
      (Class|UserWidget|RemovefromViewport (Variables|umg_menu|GetScoreHUD)))))

(event Custom|Flash
  ;[1 1 1] Flash - Flashes the screen and stops all panning on the materials, and obstacles
  (Variables|Bool|SetCanPanObstacles false)
  (Variables|Bool|SetCanInput false)
  (Variables|Bool|SetCanScore false)
  (Audio|Components|Audio|Stop (Variables|Character|GetTappyBIrd2d))
  (Utilities|FlowControl|Sequence
    (:then_0
      (bind _flash (Timeline|Timeline_Flash PlayFromStart)
        (:Update
          (Rendering|Material|SetScalarParameterValue "/Game/Materials/MPC_TappyChicken_01.MPC_TappyChicken_01" "ScreenFlashAmmount" _flash :!class /Script/Engine.KismetMaterialLibrary))))
    (:then_1
      (for _array_element (Variables|Arrays|GetActiveObstacles)
        (bind _asbp_obstacle_post_c (Utilities|Casting|CastToBP_Obstacle_Post _array_element))
        (Variables|/Game/Blueprints/BP_Obstacle_Post.BP_Obstacle_Post_C|SetCanMove _asbp_obstacle_post_c false)))))

(event Custom|Crash
  (bind _tappybird2d (Variables|Character|GetTappyBIrd2d))
  (bind _tappybird2d_2 (Variables|Character|GetTappyBIrd2d))
  ;[1 1 1] Crash - Moves the Chicken from its current location to to ground, and rotates him to point down.
  (Audio|PlaySoundatLocation "/Game/Audio/SFX_HitObstacle_01_Cue.SFX_HitObstacle_01_Cue" "0, 0, 0")
  (Collision|SetCollisionResponsetoChannel (Variables|Character|GetTappyBIrd2d) "ECC_Camera" "ECR_Ignore")
  (Components|Timeline|SetPlayRate (Variables|Default|GetTImeline_Crash) 2.0)
  (Variables|Floats|SetDeathLocation (.Z (Math|Vector|BreakVector (Transformation|GetWorldLocation _tappybird2d))))
  (Variables|Floats|SetDeathRotation (.Pitch (Class|KismetMathLibrary|BreakRot (Transformation|GetWorldRotation _tappybird2d))))
  (bind (_direction _lerplocation _lerprotation) (Timeline|TImeline_Crash PlayFromStart)
    (:Update
      (Transformation|SetWorldLocation _tappybird2d_2 (Math|Vector|MakeVector -195.0 2.9e+02 (Math|Float|Lerp (Variables|Floats|GetDeathLocation) -6.9e+02 _lerplocation)) false)
      (Transformation|SetWorldRotation _tappybird2d_2 (Class|KismetMathLibrary|MakeRot (Math|Float|Lerp (Variables|Floats|GetDeathRotation) 9e+01 _lerprotation) 0.0 0.0) false)
      ;;[1 1 1] Seeing Stars Effect
      (Effects|SpawnEmitteratLocation "/Game/Effects/SeeStars.SeeStars" (Transformation|GetWorldLocation (Variables|Character|GetTappyBIrd2d))))
    (:Finished
      (CallFunction|HitGorund))))

(event Custom|Start%20PanPowerUps
  ;[1 1 1] Power Up Collision Pickup
  (CallFunction|PanPowerUps))

(event Custom|BirdFlyInEvent
  ;[1 1 1] Retry Tappy Flyi n Starting Postion
  (Utilities|FlowControl|Sequence
    (:then_0
      (bind _tappybirdxlocation (Timeline|RetryFlyInPostion_Timeline PlayFromStart)
        (:Update
          (Transformation|SetRelativeLocation (Variables|Character|GetTappyBIrd2d) (Math|Vector|MakeVector _tappybirdxlocation 2.9e+02 0.0) false))))
    (:then_1
      (Audio|PlaySoundatLocation "/Game/Audio/SFX_Chicken_01_Cue.SFX_Chicken_01_Cue" "0, 0, 0"))))

(event Custom|PollGameCenter
  (bind _tappy2dsavegameobject (Variables|SaveGame|GetTappy2dSaveGameObject))
  ;[1 1 1] If "iOS" Check GameCenter LeaderBoard for higher score
  (bind _leaderboardvalue (|LeaderboardQuery (Game|GetPlayerController 0) "HighScore")
    (:OnSuccess
      (if (> _leaderboardvalue (Variables|scoreboard|GetHighScore))
        (Variables|scoreboard|SetHighScore _leaderboardvalue)
        (bind _asbp_tappybird2dsavegame_c (Utilities|Casting|CastToBP_TappyBIrd2dSaveGame _tappy2dsavegameobject))
        (Variables|/Game/Blueprints/BP_TappyBIrd2dSaveGame.BP_TappyBIrd2dSaveGame_C|SetHighScore _asbp_tappybird2dsavegame_c (Variables|scoreboard|GetHighScore))
        (SaveGame|SaveGametoSlot _tappy2dsavegameobject "Tappy2DSlot")))))

(event Custom|RestartHitCollisons
  (bind _tappybird2d (Variables|Character|GetTappyBIrd2d))
  (bind _tappy2dsavegameobject (Variables|SaveGame|GetTappy2dSaveGameObject))
  (bind _tappy2dsavegameobject_2 (Variables|SaveGame|GetTappy2dSaveGameObject))
  ;[1 1 1] When the Chicken hits an Obstacle and to agnore power up collision box
  (Utilities|FlowControl|Sequence
    (:then_0
      (Utilities|FlowControl|DoOnce false) ; enters at Reset
    )
    (:then_1
      (Utilities|FlowControl|DoOnce false) ; enters at Reset
    )
    (:then_2
      ;[1 1 1] Hit Ground - Opens the Scoreboard, Unhides the Play, Leaderboards, and Rate buttons, checks score to see it if beat your high score etc.
      (Utilities|FlowControl|DoOnce false) ; enters at Reset
    )))

(event Custom|FlapTappy
  ;[1 1 1] Flap - Animates the upward movement of the chicken when you tap.
  (if (Variables|Bool|GetREadyToPlay)
    (Audio|PlaySoundatLocation "/Game/Audio/SFX_FlapWing_Cue.SFX_FlapWing_Cue" "0, 0, 0")
    (bind (_direction _vertmovement _rotation) (Timeline|Timeline_0 PlayFromStart))))

(event EventBeginPlay
  (bind _returnvalue (Game|GetPlayerController 0))
  (bind _camera1 (Variables|Default|GetCamera1))
  (bind (_sizex _sizey) (HUD|GetViewportSize _returnvalue))
  ;[1 1 1] Initial Setup
  (bind _returnvalue_2 (Game|GetPlatformName))
  (Variables|Strings|SetCurrentPlatform _returnvalue_2)
  (Rendering|Material|SetScalarParameterValue "/Game/Materials/MPC_TappyChicken_01.MPC_TappyChicken_01" "FadeAmmount" 1.0 :!class /Script/Engine.KismetMaterialLibrary)
  (Utilities|FlowControl|Sequence
    (:then_0
      (bind _fade (Timeline|Timeline_FadeGameIn PlayFromStart)
        (:Update
          (Rendering|Material|SetScalarParameterValue "/Game/Materials/MPC_TappyChicken_01.MPC_TappyChicken_01" "FadeAmmount" _fade :!class /Script/Engine.KismetMaterialLibrary))))
    (:then_1
      (Utilities|FlowControl|Delay 0.2)
      ;;[1 1 1] Setup Camera
      (if (or (== _sizex 320) (== _sizex 640))
        (Variables|/Script/Engine.CameraComponent|SetOrthoWidth _camera1 1.28e+03)
        (elif (== _sizex 768)
          (Variables|/Script/Engine.CameraComponent|SetOrthoWidth _camera1 1536.0)
          (else
            (Variables|/Script/Engine.CameraComponent|SetOrthoWidth _camera1 (Math|Float|Clamp(Float) (/ (* _sizex 1.28e+03) (* _sizey 0.75)) 1.28e+03 4e+03)))))
      (Game|Player|SetViewTargetwithBlend _returnvalue self 0.0 "VTBlend_Linear" 0.0 false)
      ;[1 1 1] SaveGame
      (bind _returnvalue_3 (SaveGame|DoesSaveGameExist "Tappy2DSlot"))
      (if _returnvalue_3
        (bind _returnvalue_4 (SaveGame|LoadGamefromSlot "Tappy2DSlot"))
        (Variables|SaveGame|SetTappy2dSaveGameObject _returnvalue_4)
        (bind _asbp_tappybird2dsavegame_c (Utilities|Casting|CastToBP_TappyBIrd2dSaveGame (Variables|SaveGame|GetTappy2dSaveGameObject)))
        (Variables|scoreboard|SetHighScore (Variables|/Game/Blueprints/BP_TappyBIrd2dSaveGame.BP_TappyBIrd2dSaveGame_C|GetHighScore _asbp_tappybird2dsavegame_c))
        (Variables|Arrays|SetFoundEggs (Variables|/Game/Blueprints/BP_TappyBIrd2dSaveGame.BP_TappyBIrd2dSaveGame_C|GetFoundEggs _asbp_tappybird2dsavegame_c))
        (else
          (bind _returnvalue_5 (SaveGame|CreateSaveGameObject "/Game/Blueprints/BP_TappyBIrd2dSaveGame.BP_TappyBIrd2dSaveGame_C"))
          (Variables|SaveGame|SetTappy2dSaveGameObject _returnvalue_5)
          (bind _asbp_tappybird2dsavegame_c_2 (Utilities|Casting|CastToBP_TappyBIrd2dSaveGame (Variables|SaveGame|GetTappy2dSaveGameObject)))
          (Variables|/Game/Blueprints/BP_TappyBIrd2dSaveGame.BP_TappyBIrd2dSaveGame_C|SetHighScore _asbp_tappybird2dsavegame_c_2 0)
          (SaveGame|SaveGametoSlot (Variables|SaveGame|GetTappy2dSaveGameObject) "Tappy2DSlot")))
      ;[1 1 1] Opening Screen Tappy Fly in
      (Utilities|FlowControl|Sequence
        (:then_0
          (Utilities|Array|Clear (Variables|Arrays|GetActiveObstacles))
          (Variables|Bool|SetIsRetry false)
          (CallFunction|ResetObstacles)
          (Audio|PlaySoundatLocation "/Game/Audio/SFX_Chicken_01_Cue.SFX_Chicken_01_Cue" "0, 0, 0")
          (Rendering|SetVisibility (Variables|Sprites|Getegg) false false))
        (:then_1
          (bind _tappybirdxlocation (Timeline|Anim_ReadySCreen PlayFromStart)
            (:Update
              (Transformation|SetRelativeLocation (Variables|Character|GetTappyBIrd2d) (Math|Vector|MakeVector _tappybirdxlocation 2.9e+02 0.0) false))))
        (:then_2
          ;[1 1 1] Display Main Menu
          (bind _returnvalue_6 (Class|WidgetBlueprintLibrary|Create "/Game/Menus/MainMenu.MainMenu_C"))
          (Variables|umg_menu|SetMainMenu _returnvalue_6)
          (UserInterface|Viewport|AddtoViewport (Variables|umg_menu|GetMainMenu) false true true)
          ;[1 1 1] Start BG Track
          (Utilities|FlowControl|Delay 0.2)
          (Audio|Components|Audio|FadeIn (Variables|Default|GetBGTrack) 3.0 1.0 0.0 :!class /Script/Engine.AudioComponent))
        (:then_3
          (CallFunction|PollGameCenter))))))

(event EventTick
  (params (DeltaSeconds :type Float%20%28single-precision%29))
  (bind _tappybird2d (Variables|Character|GetTappyBIrd2d))
  ;[1 1 1] Flap - Animates the upward movement of the chicken when you tap.
  (Variables|Floats|SetDeltaTime DeltaSeconds)
  (Utilities|FlowControl|Sequence
    (:then_0
      (if (Audio|Components|Audio|IsPlaying (Variables|Character|GetTappyBIrd2d))
        (CallFunction|PanLayers))
      (if (Variables|Bool|GetCanPanObstacles)
        (CallFunction|PanObstacles))
      (if (Variables|Bool|GetREadyToPlay)
        (Transformation|SetRelativeLocation _tappybird2d (Math|Vector|MakeVector -195.0 2.9e+02 (+ (.Z (Math|Vector|BreakVector (Transformation|GetWorldLocation _tappybird2d))) (* (* (stale Custom|FlapTappy _vertmovement) 5e+02) (Variables|Floats|GetDeltaTime)))) false)
        (Transformation|SetWorldRotation _tappybird2d (Math|Interpolation|RInterpTo (Transformation|GetWorldRotation _tappybird2d) (Class|KismetMathLibrary|MakeRot (stale Custom|FlapTappy _rotation) 0.0 0.0) (Variables|Floats|GetDeltaTime) 2e+01) false)))))

(event Input|KeyboardEvents|C
  (bind _tappy2dsavegameobject (Variables|SaveGame|GetTappy2dSaveGameObject))
  ;[1 1 1] SaveGame
  (:Pressed
    (bind _asbp_tappybird2dsavegame_c (Utilities|Casting|CastToBP_TappyBIrd2dSaveGame _tappy2dsavegameobject))
    (Variables|/Game/Blueprints/BP_TappyBIrd2dSaveGame.BP_TappyBIrd2dSaveGame_C|SetHighScore _asbp_tappybird2dsavegame_c 0)
    (Variables|scoreboard|SetHighScore 0)
    (for _index (range 0 63)
      (Utilities|Array|SetArrayElem (Variables|Arrays|GetFoundEggs) _index false))
    (Variables|/Game/Blueprints/BP_TappyBIrd2dSaveGame.BP_TappyBIrd2dSaveGame_C|SetFoundEggs _asbp_tappybird2dsavegame_c (Variables|Arrays|GetFoundEggs))
    (SaveGame|SaveGametoSlot _tappy2dsavegameobject "Tappy2DSlot")
    (Development|PrintString "Saved File Has Been Cleared")))

(event Input|MouseEvents|LeftMouseButton
  ;[1 1 1] Tap Tappy Bird
  (:Pressed
    (if (Variables|Bool|GetCanInput)
      (CallFunction|FlapTappy))))

(event Input|TouchEvents|InputTouch
  (params (Location :type Vector) (FingerIndex :type ETouchIndex%20Enum))
  ;[1 1 1] Tap Tappy Bird
  (:Pressed
    (if (Variables|Bool|GetCanInput)
      (CallFunction|FlapTappy))))

(fn ConstructionScript
  (bind _returnvalue (Class|KismetSystemLibrary|MakeLiteralInteger 8))
  (bind _panninglayersprites (Variables|Arrays|GetPanningLayerSprites))
  (bind _panningobstacles (Variables|Arrays|GetPanningObstacles))
  ;[1 1 1] Panning Background Layers
  (Utilities|Array|Clear (Variables|Arrays|GetPanningLayerSprites))
  (Utilities|Array|Add _panninglayersprites (Variables|Sprites|GetCllouds))
  (Utilities|Array|Add _panninglayersprites (Variables|Sprites|GetBushes))
  (Utilities|Array|Add _panninglayersprites (Variables|Sprites|GetGround))
  (Utilities|Array|Add _panninglayersprites (Variables|Sprites|GettreesBg))
  ;[1 1 1] Panning Obstacles
  (Utilities|Array|Clear (Variables|Arrays|GetPanningObstacles))
  (Utilities|Array|Add _panningobstacles (Variables|Sprites|GetPipeTop))
  (Utilities|Array|Add _panningobstacles (Variables|Sprites|GetpipeTop2))
  (Utilities|Array|Add _panningobstacles (Variables|Sprites|GetpipeTop3))
  (Utilities|Array|Add _panningobstacles (Variables|Sprites|GetpipeTop4))
  (Utilities|Array|Add _panningobstacles (Variables|Sprites|GetpipeTop5))
  ;[1 1 1] Panning PowerUps
  (Utilities|Array|Clear (Variables|Arrays|GetPanningPowerUps))
  (Utilities|Array|Add (Variables|Arrays|GetPanningPowerUps) (Variables|Default|GetPowerUpBox))
  ;[1 1 1] Making more Dynamic material instances for items that need to change over time.
  (bind _returnvalue_2 (Rendering|Material|CreateDynamicMaterialInstance (Variables|Sprites|Getegg) 0 0 :!class /Script/Engine.PrimitiveComponent))
  (Variables|DMI|SetMID_Egg _returnvalue_2)
  (Utilities|Array|Clear (Variables|Arrays|GetMyEggCollection))
  ;[1 1 1] Create Found Eggs
  (for _index (range 0 63)
    (bind _returnvalue_3 (AddComponent|AddPaperSpriteComponent false))
    (Utilities|Array|Add (Variables|Arrays|GetMyEggCollection) _returnvalue_3)
    (bind _returnvalue_4 (Rendering|Material|CreateDynamicMaterialInstance _returnvalue_3 0 0 :!class /Script/Engine.PrimitiveComponent))
    (Rendering|Material|SetScalarParameterValue _returnvalue_4 "FrameNumber" (Math|Conversions|ToFloat(Integer) _index) :!class /Script/Engine.MaterialInstanceDynamic)
    (Transformation|SetRelativeLocation _returnvalue_3 (Math|Vector|MakeVector -2.0 (- (* (Math|Conversions|ToFloat(Integer) (Math|Integer|%(Integer) _index _returnvalue)) 232.0) (* 99.0 8.0)) (+ (Math|Conversions|ToFloat(Integer) (* (Math|Integer|%(Integer) _index _returnvalue) -280)) (* 123.0 8.0))) false)
    (Rendering|SetVisibility _returnvalue_3 false false)))

(fn PanObstacles
  (bind _canobstaclescore (Variables|Arrays|GetCanObstacleScore))
  (for (_array_element _array_index) (Variables|Arrays|GetPanningObstacles)
    (if (< (.X (Math|Vector|BreakVector (Variables|/Script/Engine.SceneComponent|GetRelativeLocation _array_element))) -195.0)
      (if (Utilities|Array|Get(acopy) _canobstaclescore _array_index)
        (Utilities|Array|SetArrayElem _canobstaclescore _array_index false)
        (CallFunction|Score)))
    (if (< (.X (Math|Vector|BreakVector (Variables|/Script/Engine.SceneComponent|GetRelativeLocation _array_element))) -2e+03)
      (Utilities|Array|SetArrayElem (Variables|Arrays|GetCanObstacleScore) _array_index true)
      (Transformation|AddRelativeLocation _array_element "4000.000000,170.000000, 0" false)
      (Transformation|SetRelativeLocation _array_element (Math|Vector|MakeVector (.X (Math|Vector|BreakVector (Variables|/Script/Engine.SceneComponent|GetRelativeLocation _array_element))) 1.7e+02 (+ 3.1e+02 (Math|Random|RandomFloatinRange -256.0 256.0))) false))
    (Transformation|AddRelativeLocation _array_element (Math|Vector|MakeVector (* (* (* 0.08 (Variables|Floats|GetDeltaTime)) 4e+03) -1.0) 0.0 0.0) false)))

(fn PanLayers
  (for (_array_element _array_index) (Variables|Arrays|GetPanningLayerSprites)
    (if (< (.X (Math|Vector|BreakVector (Variables|/Script/Engine.SceneComponent|GetRelativeLocation _array_element))) -4096.0)
      (Transformation|AddRelativeLocation _array_element "4096.000000, 0, 0" false))
    (Transformation|AddRelativeLocation _array_element (Math|Vector|MakeVector (* (* (* (Utilities|Array|Get(acopy) (Variables|Arrays|GetPanningLayerTimes) _array_index) (Variables|Floats|GetDeltaTime)) 4e+03) -1.0) 0.0 0.0) false)))

(fn ResetObstacles
  (bind _canobstaclescore (Variables|Arrays|GetCanObstacleScore))
  (for (_array_element _array_index) (Variables|Arrays|GetPanningObstacles)
    (Transformation|SetRelativeLocation _array_element (Math|Vector|MakeVector (Math|Conversions|ToFloat(Integer) (+ 3072 (* _array_index 800))) 1.7e+02 (+ 3.1e+02 (Math|Random|RandomFloatinRange -256.0 256.0))) false))
  (for (_ _array_index_2) _canobstaclescore
    (Utilities|Array|SetArrayElem _canobstaclescore _array_index_2 true)))

(fn ChooseSkyColor
  (LocalVariables|SetNewSkyColor (Math|Random|RandomIntegerinRange 0 3) :!label _label)
  (if (!= (Variables|Int|GetCurrentSkyColor) (LocalVariables|GetNewSkyColor))
    (Variables|Int|SetCurrentSkyColor (LocalVariables|GetNewSkyColor))
    (switch int (Variables|Int|GetCurrentSkyColor)
      (:0
        (CallFunction|SetSkyColor "(R=0.000000,G=0.490196,B=0.878000,A=1.000000)"))
      (:1
        (CallFunction|SetSkyColor "(R=0.750000,G=0.377000,B=0.516000,A=1.000000)"))
      (:2
        (CallFunction|SetSkyColor "(R=0.065333,G=0.418682,B=0.525000,A=1.000000)"))
      (:3
        (CallFunction|SetSkyColor "(R=0.024000,G=0.195000,B=0.176000,A=1.000000)")))
    (else
      (goto _label))))

(fn SetSkyColor
  (params (SkyColor :type Linear%20Color%20Structure))
  (Sprite|SetSpriteColor (Variables|Sprites|GetBackground) SkyColor))

(fn ChoosePowerUp
  (LocalVariables|SetNewPowerUp (Math|Random|RandomIntegerinRange 0 3) :!label _label)
  (if (!= (Variables|Int|GetCurrentPowerUp) (LocalVariables|GetNewPowerUp))
    (Variables|Int|SetCurrentPowerUp (LocalVariables|GetNewPowerUp))
    (switch int (Variables|Int|GetCurrentPowerUp)
      (:0
        (CallFunction|SetPowerUp "/Game/Textures/powerupCube_Sprite.powerupCube_Sprite")
        (Development|PrintString "0"))
      (:1
        (CallFunction|SetPowerUp "/Game/Textures/powerupB_Sprite.powerupB_Sprite")
        (Development|PrintString "1"))
      (:2
        (CallFunction|SetPowerUp "/Game/Textures/powerupY_Sprite.powerupY_Sprite")
        (Development|PrintString "2"))
      (:3
        (CallFunction|SetPowerUp "/Game/Textures/powerupP_Sprite.powerupP_Sprite")
        (Development|PrintString "3")))
    (else
      (goto _label))))

(fn SetPowerUp
  (params (PowerUpType :type Paper%20Sprite%20Object%20Reference))
  (Rendering|Components|Sprite|SetSprite (Variables|Default|GetPowerUpBox) PowerUpType))

(fn PanPowerUps
  (for (_array_element _array_index) (Variables|Arrays|GetPanningPowerUps)
    (if (< (.X (Math|Vector|BreakVector (Variables|/Script/Engine.SceneComponent|GetRelativeLocation _array_element))) -3.5e+02)
      _
      (else
        _))
    (if (< (.X (Math|Vector|BreakVector (Variables|/Script/Engine.SceneComponent|GetRelativeLocation _array_element))) -2e+03)
      (Transformation|AddRelativeLocation _array_element "4342.000000,228.000000,0.000000" false)
      (Transformation|SetRelativeLocation _array_element (Math|Vector|MakeVector (.X (Math|Vector|BreakVector (Variables|/Script/Engine.SceneComponent|GetRelativeLocation _array_element))) 228.0 (+ 3.1e+02 (Math|Random|RandomFloatinRange -256.0 256.0))) false))
    (Transformation|AddRelativeLocation _array_element (Math|Vector|MakeVector (* (* (* 0.08 (Variables|Floats|GetDeltaTime)) 4e+03) -1.0) 0.0 0.0) false)))

(fn ResetPowerUps
  (for (_array_element _array_index) (Variables|Arrays|GetPanningPowerUps)
    (Transformation|SetRelativeLocation _array_element (Math|Vector|MakeVector (Math|Conversions|ToFloat(Integer) (+ 4000 (* _array_index 800))) 228.0 (+ 3.1e+02 (Math|Random|RandomFloatinRange -256.0 256.0))) false)))